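; BP_ScreenCaptureRecorder records the desktop to an MP4 video for as long as it is in play.
; On BeginPlay it launches a bundled ffmpeg.exe as a hidden process, using gdigrab to capture the desktop.
; The output file goes to the video path, named by concatenating the current date and time.
; EndPlay calls StopRecorder, which closes the process, then runs the parent EndPlay.
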(event `self.ReceiveBeginPlay`
  (`self.StartRecorder`))

(event `StartRecorder`
  (bind (_returnvalue_year _returnvalue_month _returnvalue_day _returnvalue_hour _returnvalue_minute _returnvalue_second) (`KismetMathLibrary.BreakDateTime` (`KismetMathLibrary.Now`)))
  (`self.Launch` (`KismetStringLibrary.Concat_StrStr` (`self.GetAddtionAssetPath`) "/ffmpeg.exe") (`KismetStringLibrary.Concat_StrStr` "-f gdigrab -i desktop -pix_fmt yuv420p " (`self.GetVideoPath`) "/" (`KismetStringLibrary.Concat_StrStr` (`KismetStringLibrary.Conv_IntToString` _returnvalue_year) (`KismetStringLibrary.Conv_IntToString` _returnvalue_month) (`KismetStringLibrary.Conv_IntToString` _returnvalue_day) (`KismetStringLibrary.Conv_IntToString` _returnvalue_hour) (`KismetStringLibrary.Conv_IntToString` _returnvalue_minute) (`KismetStringLibrary.Conv_IntToString` _returnvalue_second)) ".mp4") true))

(event `StopRecorder`
  (`self.CloseProcess`))

(event `self.ReceiveEndPlay`
  (params (EndPlayReason :type "EEndPlayReason Enum" :default "Destroyed"))
  (`self.StopRecorder`)
  (`parent.ReceiveEndPlay` EndPlayReason))

(fn `UserConstructionScript`)